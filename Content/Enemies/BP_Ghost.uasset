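; Ghost enemy that takes damage and is destroyed when its hitpoints reach zero.
; Each tick it yaws along the camera-to-ghost direction to keep its sprite aligned to the player's view.
; Overlapping a player-controlled pawn reloads the FirstPersonMap level, a stopgap until player death exists.
; A damage-over-time function for pawns overlapping its capsule exists but is currently not wired to run.
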(event `self.ReceiveActorBeginOverlap`
  (params (OtherActor :type "Actor Object Reference"))
  ; Simple workaround to restart the level until there's a proper damage/death system for the player
  (bind _aspawn (cast `Pawn` OtherActor))
  (if (`self.IsPlayerControlled` _aspawn)
    (`GameplayStatics.OpenLevel` "FirstPersonMap")))

(event `self.ReceiveTick`
  (params (DeltaSeconds :type "Float (single-precision)"))
  (`self.UpdateSpriteAlignment`))

(event `self.ReceiveAnyDamage`
  (params (Damage :type "Float (single-precision)") (DamageType :type "DamageType Object Reference") (InstigatedBy :type "Controller Object Reference") (DamageCauser :type "Actor Object Reference"))
  (bind _output_get (set `self.Hitpoints` (- (`self.Hitpoints`) Damage)))
  (if (<= _output_get 0.0)
    (`self.K2_DestroyActor`)))

(fn `HandleDamage`
  (params (DeltaSeconds :type "Float (double-precision)"))
  (for _array_element (`PrimitiveComponent.GetOverlappingActors` (`self.CapsuleComponent`) "/Script/Engine.Pawn")
    (`GameplayStatics.ApplyDamage` _array_element (* DeltaSeconds (`self.DamagePerSecond`)))))

(fn `UpdateSpriteAlignment`
  (bind (_returnvalue_roll _returnvalue_pitch _returnvalue_yaw) (`KismetMathLibrary.BreakRotator` (`KismetMathLibrary.FindLookAtRotation` (`PlayerCameraManager.GetCameraLocation` (`GameplayStatics.GetPlayerCameraManager` 0)) (`self.K2_GetActorLocation`))))
  (`self.K2_SetActorRotation` (`KismetMathLibrary.MakeRotator` 0.0 0.0 _returnvalue_yaw)))

(fn `UserConstructionScript`)